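; BP_GenerateMap is a map actor with a test input that edits its map where the mouse clicks.
; The click line-traces from the cursor, and on a hit against this actor class a new ProceduralBrushTool applies a circle brush at the hit's XY.
; UpdateMap then receives the edited Map.
; The construction script is empty, and GetPosition and SetSquare hold only unused grid index and quad-corner math.
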(event `InputAction|Click`
  (params (Key :type "Key Structure" :default "AnyKey"))
  (bind __map (`self._Map`))
  (bind (_worldlocation _worlddirection) (`PlayerController.DeprojectMousePositionToWorld` (`GameplayStatics.GetPlayerController` 0)))
  ;[1 1 1] Test
  (:`Pressed`
    (bind _outhit (`KismetSystemLibrary.LineTraceSingle` :`Start` _worldlocation :`End` (+ _worldlocation (* _worlddirection (`self.SightDistance`))) :`TraceChannel` "TraceTypeQuery3" :`DrawDebugType` "Persistent" :`bIgnoreSelf` false))
    (bind (_bblockinghit _binitialoverlap _time _location _impactpoint _normal _impactnormal _physmat _hitactor) (`GameplayStatics.BreakHitResult` _outhit))
    (cast `/Game/BP/BP_GenerateMap` _hitactor)
    (bind _returnvalue (`|GenericCreateObject` "/Script/ProceduralMap.ProceduralBrushTool" self))
    (`ProceduralBrushTool.CircleBrush` _returnvalue (`KismetMathLibrary.MakeVector2D` (.x _location) (.y _location)) 100.0 10 __map)
    (`self.UpdateMap` __map)))

(fn `UserConstructionScript`)