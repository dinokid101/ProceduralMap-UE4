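; Procedural mesh actor that builds a flat, grass-textured grid of SizeX by SizeY squares on BeginPlay.
; MakeSquare emits six unshared vertices per cell with fixed UVs and -Y normals, appended into arrays for one mesh section with sequential triangle indices.
; The index loop runs to the array length, apparently one index too many.
; Height support is unfinished: HeightMap is never applied, and MakeMesh and DebugMesh helpers are never called.
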(event EventBeginPlay
  (Variables|Default|SetHeightMap (Utilities|Array|MakeArray 1 1 1 1 1 0 0 0 0 0 0 0 0 0 0 0))
  (for _index (range 0 (- (Variables|Default|Getsize_y) 1))
    (Variables|Default|Seti _index)
    (for _index_2 (range 0 (- (Variables|Default|Getsize_x) 1))
      (Variables|Default|Setj _index_2)
      (bind (_verticesarray _uv _newparam) (CallFunction|MakeSquare (Variables|Default|Getj) (Variables|Default|Geti) 1e+02))
      (Utilities|Array|AppendArray (Variables|Default|GetVerticesArray) _verticesarray)
      (Utilities|Array|AppendArray (Variables|Default|GetUV) _uv)
      (Utilities|Array|AppendArray (Variables|Default|GetNormalArray) _newparam)))
  (Utilities|FlowControl|Sequence
    (:then_0
      (for _index_3 (range 0 (Utilities|Array|Length (Variables|Default|GetVerticesArray)))
        (Utilities|Array|Add (Variables|Default|GetTriangleArray) _index_3)))
    (:then_1
      (Rendering|Material|SetMaterial (Variables|Default|GetProceduralMesh) 0 "/Game/StarterContent/Materials/M_Ground_Grass.M_Ground_Grass"))
    (:then_2
      (Class|ProceduralMeshComponent|CreateMeshSectionLinearColor (Variables|Default|GetProceduralMesh) 0 (Variables|Default|GetVerticesArray) (Variables|Default|GetTriangleArray) (Variables|Default|GetNormalArray) (Variables|Default|GetUV) 0 0 false))))

(fn ConstructionScript)

(fn MakeMesh
  (params (V1 :type Vector) (V2 :type Vector) (V3 :type Vector) (VerticesArray :type Array%20of%20Vectors) (NormalArray :type Array%20of%20Vectors) (TriangleArray :type Array%20of%20Integers))
  (LocalVariables|SetLocalVerticesArray VerticesArray)
  (LocalVariables|SetLocalNormalArray NormalArray)
  (LocalVariables|SetLocalTriangleArray TriangleArray)
  ;[1 1 1] Adds vertices to the array
  (Utilities|Array|Add (LocalVariables|GetLocalVerticesArray) V1)
  (Utilities|Array|Add (LocalVariables|GetLocalVerticesArray) V2)
  (bind _returnvalue (Utilities|Array|Add (LocalVariables|GetLocalVerticesArray) V3))
  (for _index (range (- _returnvalue 2) _returnvalue)
    ;[1 1 1] Compute normals
    (Utilities|Array|Add (LocalVariables|GetLocalNormalArray) (Math|Vector|Normalize (Utilities|Array|Get(acopy) (LocalVariables|GetLocalVerticesArray) _index)))
    ;[1 1 1] Adds triangle index
    (Utilities|Array|Add (LocalVariables|GetLocalTriangleArray) _index))
  (return (LocalVariables|GetLocalVerticesArray) (LocalVariables|GetLocalNormalArray) (LocalVariables|GetLocalTriangleArray)))

(fn MakeSquare
  (params (XIndex :type Integer) (YIndex :type Integer) (Scale :type Float%20%28single-precision%29))
  (bind _localverticesarray (LocalVariables|GetLocalVerticesArray))
  (Utilities|FlowControl|Sequence
    (:then_0
      (LocalVariables|SetLocal_J XIndex)
      (LocalVariables|SetLocal_I YIndex)
      (LocalVariables|SetLocalScale (Math|Float|Truncate Scale)))
    (:then_1
      (LocalVariables|SetA 0))
    (:then_3
      (Utilities|Array|Add _localverticesarray (Math|Vector|MakeVector (Math|Conversions|ToFloat(Integer) (+ (* (LocalVariables|GetLocalScale) (LocalVariables|GetLocal_J)) (LocalVariables|GetLocalScale))) (Math|Conversions|ToFloat(Integer) (* (LocalVariables|GetLocalScale) (LocalVariables|GetLocal_I))) (Math|Conversions|ToFloat(Integer) (* (LocalVariables|Getb) (LocalVariables|GetLocalScale)))))
      (Utilities|Array|Add _localverticesarray (Math|Vector|MakeVector (Math|Conversions|ToFloat(Integer) (* (LocalVariables|GetLocalScale) (LocalVariables|GetLocal_J))) (Math|Conversions|ToFloat(Integer) (* (LocalVariables|GetLocalScale) (LocalVariables|GetLocal_I))) (Math|Conversions|ToFloat(Integer) (* (LocalVariables|GetA) (LocalVariables|GetLocalScale)))))
      (Utilities|Array|Add _localverticesarray (Math|Vector|MakeVector (Math|Conversions|ToFloat(Integer) (* (LocalVariables|GetLocalScale) (LocalVariables|GetLocal_J))) (Math|Conversions|ToFloat(Integer) (+ (* (LocalVariables|GetLocalScale) (LocalVariables|GetLocal_I)) (LocalVariables|GetLocalScale))) (Math|Conversions|ToFloat(Integer) (* (LocalVariables|Getc) (LocalVariables|GetLocalScale)))))
      (Utilities|Array|Add _localverticesarray (Math|Vector|MakeVector (Math|Conversions|ToFloat(Integer) (* (LocalVariables|GetLocalScale) (LocalVariables|GetLocal_J))) (Math|Conversions|ToFloat(Integer) (+ (* (LocalVariables|GetLocalScale) (LocalVariables|GetLocal_I)) (LocalVariables|GetLocalScale))) 0.0))
      (Utilities|Array|Add _localverticesarray (Math|Vector|MakeVector (Math|Conversions|ToFloat(Integer) (+ (* (LocalVariables|GetLocalScale) (LocalVariables|GetLocal_J)) (LocalVariables|GetLocalScale))) (Math|Conversions|ToFloat(Integer) (+ (* (LocalVariables|GetLocalScale) (Variables|Default|Geti)) (LocalVariables|GetLocalScale))) (Math|Conversions|ToFloat(Integer) (* (LocalVariables|Getd) (LocalVariables|GetLocalScale)))))
      (Utilities|Array|Add _localverticesarray (Math|Vector|MakeVector (Math|Conversions|ToFloat(Integer) (+ (* (LocalVariables|GetLocalScale) (LocalVariables|GetLocal_J)) (LocalVariables|GetLocalScale))) (Math|Conversions|ToFloat(Integer) (* (LocalVariables|GetLocalScale) (LocalVariables|GetLocal_I))) 0.0))
      (return (LocalVariables|GetLocalVerticesArray) (Utilities|Array|MakeArray "(X=1.000000,Y=0.000000)" "" "(X=0.000000,Y=1.000000)" "(X=0.000000,Y=1.000000)" "(X=1.000000,Y=1.000000)" "(X=1.000000,Y=0.000000)") (Utilities|Array|MakeArray "0,-1.000000, 0" "0,-1.000000, 0" "0,-1.000000, 0" "0,-1.000000, 0" "0,-1.000000, 0" "0,-1.000000, 0")))))